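; Steam ejector machine that turns reactor steam pressure into an incondensable extraction flow for other machines to read.
; Each Tick pulls pressure from ReactorTarget and linearly maps it between minimum and maximum working pressures to a clamped flow, served through MachinePull.
; Switch input sets EjectorState, which is sent to the display targets on change and at BeginPlay.
; The switch state does not affect the computed flow.
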(event `self.ReceiveBeginPlay`
  (`self.RefreshDisplay`))

(event `/Game/MachineBlueprints/MachineInterface.InputStateSwitch`
  (params (State :type Boolean))
  (bind _output_get (set `self.EjectorState` State))
  (for _array_element (`self.StateDisplayTargets`)
    (message `/Game/MachineBlueprints/MachineInterface.DisplayState` _array_element _output_get)))

(event `self.ReceiveTick`
  (params (DeltaSeconds :type "Float (single-precision)"))
  (bind _incondensablemaxflow (`self.IncondensableMaxflow`))
  (bind _minimumworkingpressure (`self.MinimumWorkingpressure`))
  ;[1 1 1] Get Flow
  (if true
    (bind (_integerdata _floatdata) (message `/Game/MachineBlueprints/MachineInterface.MachinePull` (`self.ReactorTarget`)))
    (bind _output_get (set `self.SteamPressure` _floatdata))
    (set `self.EjectorIncondensableFlow` (`KismetMathLibrary.FClamp` (`KismetMathLibrary.Lerp` 0.0 _incondensablemaxflow (/ (- _output_get _minimumworkingpressure) (- (`self.MaxWorkingPressure`) _minimumworkingpressure))) 0.0 _incondensablemaxflow))))

(fn `MachinePull`
  (returns (IntegerData :type Integer) (FloatData :type "Float (double-precision)") (FloatData2 :type "Float (double-precision)") (BoolData :type Boolean) (`Float Data 3` :type "Float (double-precision)"))
  (return 0 (`self.EjectorIncondensableFlow`) 0.0 false 0.0))

(fn `RefreshDisplay`
  (for _array_element (`self.StateDisplayTargets`)
    (message `/Game/MachineBlueprints/MachineInterface.DisplayState` _array_element (`self.EjectorState`))))

(fn `UserConstructionScript`)