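; Nuclear reactor machine that simulates control rods, water level and safety relief, pushing readings to display targets.
; Valve and rod events set state, and a Delay loop steps nine rods' insertion and meshes.
; Tick adds feedwater through the isolation valve, vents on overfill via a latched relief flag, and updates rod flux.
; Rod power, boiling and steam pressure logic is present but unconnected, though MachinePull returns steam pressure.
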(event `self.ReceiveBeginPlay`
  ;[1 1 1] Setup Array
  (set `self.ControlRodObjects` (`|MakeArray` (`self.ControlRod1`) (`self.ControlRod2`) (`self.ControlRod3`) (`self.ControlRod4`) (`self.ControlRod5`) (`self.ControlRod6`) (`self.ControlRod7`) (`self.ControlRod8`) (`self.ControlRod9`)))
  (`self.DisplayRefresh`))

(event `/Game/MachineBlueprints/MachineInterface.ReactorCrossoverValvePush`
  (params (NewCrossoverState :type Boolean))
  (bind _output_get (set `self.CrossoverValve` NewCrossoverState))
  (for _array_element (`self.CrossoverStateDisplayTargets`)
    (message `/Game/MachineBlueprints/MachineInterface.DisplayStatePush` _array_element _output_get)))

(event `/Game/MachineBlueprints/MachineInterface.ReactorIsolationValvePush`
  (params (ValveState :type Boolean))
  (bind _output_get (set `self.IsolationValveState` ValveState))
  (for _array_element (`self.IsolationValveStateDisplayTarget`) :!label _label
    (message `/Game/MachineBlueprints/MachineInterface.DisplayStatePush` _array_element _output_get)))

(event `DisplayRefresh`
  (goto _label))

(event `/Game/MachineBlueprints/MachineInterface.ReactorRodMovePush`
  (params (Direction :type Integer))
  (bind _controlrodperin (`self.ControlRodPerIn`))
  (bind _controlrodspeedsetting (`self.ControlRodSpeedSetting`))
  ;[1 1 1] Control Rod Movement
  (bind _output_get (set `self.ControlRodSpeedSetting` Direction))
  (if (not (== _output_get 2)) :!label _label_2
    (for (_array_element _array_index) _controlrodperin
      (bind _returnvalue (> _output_get 2))
      (if (not (or (and (>= _array_element 100.0) _returnvalue) (and (not _returnvalue) (<= _array_element 0.0))))
        (`KismetArrayLibrary.Array_Set` _controlrodperin _array_index (+ _array_element (* (`KismetMathLibrary.SelectFloat` (`self.ControlRodSpeedLow`) (`self.ControlRodSpeedHigh`) (or (== _controlrodspeedsetting 1) (== _controlrodspeedsetting 3))) (`KismetMathLibrary.SelectFloat` 1.0 -1.0 _returnvalue))))
        (bind _output (`|GetArrayItem` (`self.ControlRodObjects`) _array_index))
        (bind (_relativelocation_x _relativelocation_y) (`KismetMathLibrary.BreakVector` (`SceneComponent.RelativeLocation` _output)))
        (`SceneComponent.K2_SetRelativeLocation` _output (`KismetMathLibrary.MakeVector` _relativelocation_x _relativelocation_y (`KismetMathLibrary.Lerp` -70.0 -10.0 (/ _array_element 100.0))) false false)
        (`KismetSystemLibrary.Delay` 0.01)
        (goto _label_2)))))

(event `self.ReceiveTick`
  (params (DeltaSeconds :type "Float (single-precision)"))
  (bind _controlrodflux (`self.ControlRodFlux`))
  (bind _reactorwaterlevelmin (`self.ReactorWaterLevelMin`))
  (bind _maximumwateramount (`self.MaximumWaterAmount`))
  (bind _steamamountkg (`self.SteamAmountKg`))
  ;[1 1 1] Water Input
  (message `/Game/MachineBlueprints/MachineInterface.MachinePull` (`self.FeedwaterRegulationValveTarget`)) ; ValveKGin
  (if (`self.IsolationValveState`)
    (bind _output_get (set `self.FeedwaterKGEntry` (`self.FeedwaterKGEntry`)))
    (bind _output_get_2 (set `self.ReactorWaterKG` (+ _output_get (`self.ReactorWaterKG`)))))
  ;[1 1 1] Water Level Calculation
  (bind _output_get_3 (set `self.ReactorLevel` (`KismetMathLibrary.Lerp` -5.0 3.0 (/ (`KismetMathLibrary.FClamp` (- _output_get_2 _reactorwaterlevelmin) 0.0 _maximumwateramount) (- _maximumwateramount _reactorwaterlevelmin)))))
  (message `/Game/MachineBlueprints/MachineInterface.DisplayFloatPush` (`self.LevelDisplayTarget`) _output_get_3)
  (message `/Game/MachineBlueprints/MachineInterface.DisplayFloatPush` (`self.ReactorWaterKGDisplayTarget`) (`self.ReactorWaterKG`))
  ;[1 1 1] Safety Relief Valve
  (if (> (`self.ReactorWaterKG`) (`self.MaximumWaterAmount`))
    (bind _output_get_4 (set `self.DrumSafetyReliefState` true)))
  (if _output_get_4
    (if (> (`self.ReactorWaterKG`) (* (`self.MaximumWaterAmount`) 0.1))
      (set `self.ReactorWaterKG` (- (`self.ReactorWaterKG`) (`self.DrumSafetyReliefFlow`)))
      (set `self.SteamAmountKg` (- _steamamountkg (* _steamamountkg (`self.PressureSafetyMultiplier`))))
      ;[1 1 1] Change Flux With Flux Rate
      (for (_array_element _array_index) (`self.ControlRodFluxRate`) :!label _label_3
        (`KismetArrayLibrary.Array_Set` _controlrodflux _array_index (* _array_element (`|GetArrayItem` _controlrodflux _array_index)))
        ;[1 1 1] Display Control Rod Data
        (for (_array_element_2 _array_index_2) (`self.ControlRodLevelDisplayTarget`)
          (message `/Game/MachineBlueprints/MachineInterface.DoubleFloatDisplayPush` _array_element_2 (`|GetArrayItem` (`self.ControlRodPerIn`) _array_index_2) (`|GetArrayItem` (`self.ControlRodFlux`) _array_index_2)))))
    (else
      (goto _label_3))))

(fn `MachinePull`
  (returns (IntegerData :type Integer) (FloatData :type "Float (double-precision)") (FloatData2 :type "Float (double-precision)"))
  (return 0 (`self.SteamPressureKPa`) 0.0))

(fn `UserConstructionScript`)