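; Condenser machine that simulates condenser pressure, steam condensing and water level for a turbine system.
; Tick pulls ejector, circulation pump and turbine flows, updating steam, foreign gas, pressure and water inside the pump loop.
; Selector input ramps the bypass valve through a Delay loop; relief valve input vents gas; both update displays via message calls.
; MachinePull exposes pressure and boost state, which engages when circulation is insufficient for incoming steam.
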(event `/Game/MachineBlueprints/MachineInterface.InputSpeedIntegerSelector`
  (params (ValveStateSelector :type Integer))
  ;[1 1 1] CondenserBypassControl
  (if (== ValveStateSelector 0) :!label _label
    (set `self.BypassValve` (`KismetMathLibrary.FClamp` (- (`self.BypassValve`) (`self.BypassValveSelectorSpeed`))))
    (for _array_element (`self.BypassValveDisplayTargets`) :!label _label_2
      (message `/Game/MachineBlueprints/MachineInterface.DisplayFloat` _array_element (* (`self.BypassValve`) 100.0)))
    (`KismetSystemLibrary.Delay` 0.1)
    (goto _label)
    (elif (== ValveStateSelector 2)
      (set `self.BypassValve` (`KismetMathLibrary.FClamp` (+ (`self.BypassValve`) (`self.BypassValveSelectorSpeed`))))
      (goto _label_2))))

(event `self.ReceiveBeginPlay`
  (`self.RefreshDisplay`))

(event `/Game/MachineBlueprints/MachineInterface.InputCondenserSafetyReliefValve`
  (params (`Valve State` :type Boolean))
  ;[1 1 1] Safety Relief Valve Input
  (bind _output_get (set `self.SafetyReliefValveState` `Valve State`))
  (for _array_element (`self.SafetyReliefValveStateDisplayTargets`)
    (message `/Game/MachineBlueprints/MachineInterface.DisplayState` _array_element _output_get)))

(event `self.ReceiveTick`
  (params (DeltaSeconds :type "Float (single-precision)"))
  (bind _returnvalue (+ (`self.WaterAmount`) (`self.SteamCondensingAmount`)))
  ;[1 1 1] Set Ejector flows
  (bind (_integerdata _floatdata) (message `/Game/MachineBlueprints/MachineInterface.MachinePull` (`self.Ejector 1 Target`)))
  (set `self.Ejector 1 Flow` _floatdata)
  (bind (_integerdata_2 _floatdata_2) (message `/Game/MachineBlueprints/MachineInterface.MachinePull` (`self.Ejector 2 Target`)))
  (set `self.Ejector 2 Flow` _floatdata_2)
  ;[1 1 1] Set Circulation Flow
  (set `self.CirculationFlow` 0.0)
  (for _array_element (`self.CirculationPumpTargets`)
    (bind (_integerdata_3 _floatdata_3) (message `/Game/MachineBlueprints/MachineInterface.MachinePull` _array_element))
    (bind _output_get (set `self.CirculationFlow` (+ _floatdata_3 (`self.CirculationFlow`))))
    (set `self.BoostedCircFLow` (* _output_get (`self.BoostStateMultiplier`)))
    ;[1 1 1] Safety Relief Valve Check
    (if (`self.SafetyReliefValveState`)
      (set `self.SafetyReliefValveFlow` 200.0)
      (set `self.SafetyReliefValveForeignFlow` 160.0)
      (else
        (set `self.SafetyReliefValveFlow` 0.0)
        (set `self.SafetyReliefValveForeignFlow` 0.0)))
    ;[1 1 1] Get Steam coming in
    (bind (_integerdata_4 _floatdata_4) (message `/Game/MachineBlueprints/MachineInterface.MachinePull` (`self.TurbineTarget`)))
    (bind _output_get_2 (set `self.SteamIn` (+ _floatdata_4 (`KismetMathLibrary.Lerp` 0.0 (`self.Bypass100%Flow`) (`self.BypassValve`)))))
    (if (< (/ (* _output_get_2 (`self.CirculationFlowFor100%`)) (`self.SteamCondensingAmountNominal100%`)) (`self.CirculationFlow`))
      ;[1 1 1] Calculate Amount of steam that gets condensed
      (set `self.BoostState` false)
      (set `self.SteamCondensingAmount` (* (`self.SteamCondensingAmountNominal100%`) (/ (`self.CirculationFlow`) (`self.CirculationFlowFor100%`))))
      (else
        ;[1 1 1] SteamCondensingWithBoost
        (set `self.BoostState` true)
        (set `self.SteamCondensingAmount` (* (`self.SteamCondensingAmountNominal100%`) (/ (* (`self.CirculationFlow`) (`self.BoostStateMultiplier`)) (`self.CirculationFlowFor100%`))))))
    ;[1 1 1] SetSteamGasAmount
    (set `self.Steamgas` (+ (`self.Steamgas`) (- (`self.SteamIn`) (`self.SteamCondensingAmount`) (`self.SafetyReliefValveFlow`))))
    ;[1 1 1] Set foreign gas amount
    (set `self.Foreigngas` (`KismetMathLibrary.FClamp` (- (+ (`self.Foreigngas`) (`self.SafetyReliefValveForeignFlow`) (`self.ForeignGasDefaultGain`)) (`self.Ejector 1 Flow`) (`self.Ejector 2 Flow`)) 5346.0 (`self.TotalGasPress101kpa`)))
    ;[1 1 1] Set Pressure
    (bind _output_get_3 (set `self.TotalGas` (+ (`self.Foreigngas`) (`self.Steamgas`))))
    (set `self.CondenserPressure` (`KismetMathLibrary.Lerp` 0.0 101.0 (/ _output_get_3 (`self.TotalGasPress101kpa`))))
    ;[1 1 1] Set Water Amount and Level
    (if (>= _returnvalue 0.0)
      (bind _output_get_4 (set `self.WaterAmount` _returnvalue))
      (else
        (set `self.WaterAmount` 0.0)))
    (set `self.WaterLevel` (`KismetMathLibrary.Lerp` 3.5 -4.0 (/ _output_get_4 (`self.WaterAmountMax`))))))

(fn `DisplayState`
  (params (StatePushed :type Boolean))
  (return))

(fn `MachinePull`
  (returns (IntegerData :type Integer) (FloatData :type "Float (double-precision)") (FloatData2 :type "Float (double-precision)") (BoolData :type Boolean) (`Float Data 3` :type "Float (double-precision)") (`Float Data 4` :type "Float (double-precision)"))
  (return 0 (`self.CondenserPressure`) 0.0 (`self.BoostState`) 0.0 0.0))

(fn `RefreshDisplay`
  (for _array_element (`self.SafetyReliefValveStateDisplayTargets`)
    (message `/Game/MachineBlueprints/MachineInterface.DisplayState` _array_element (`self.SafetyReliefValveState`))))

(fn `UserConstructionScript`)