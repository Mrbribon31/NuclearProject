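; Coolant water circulation pump machine that simulates valve, pump and boost states plus water fill level, mirroring them to linked displays.
; Input events set valve and pump states, while Tick pulls boost from the condenser and fills or drains water when only one valve is open.
; Nominal flow latches once full, running and both valves open, exposed through MachinePull; nothing resets it.
; The inlet valve event always sends false to its displays.
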(event `/Game/MachineBlueprints/MachineInterface.InputLargePumpValveOut`
  (params (OutValveState :type Boolean))
  (bind _output_get (set `self.ValveOutState` OutValveState))
  (for _array_element (`self.ValveOutStateDisplayTarget`)
    (message `/Game/MachineBlueprints/MachineInterface.DisplayState` _array_element _output_get)))

(event `/Game/MachineBlueprints/MachineInterface.InputLargePumpValveIn`
  (params (InValveState :type Boolean))
  (set `self.InputValveState` InValveState)
  (for _array_element (`self.ValveInStateDisplayTarget`)
    (message `/Game/MachineBlueprints/MachineInterface.DisplayState` _array_element false)))

(event `/Game/MachineBlueprints/MachineInterface.InputStateSwitch`
  (params (State :type Boolean))
  (bind _output_get (set `self.PumpState` State))
  (for _array_element (`self.PumpStateDisplayTarget`)
    (message `/Game/MachineBlueprints/MachineInterface.DisplayState` _array_element _output_get)))

(event `self.ReceiveTick`
  (params (DeltaSeconds :type "Float (single-precision)"))
  ;[1 1 1] BoostStateControl
  (bind (_integerdata _floatdata _floatdata2 _booldata) (message `/Game/MachineBlueprints/MachineInterface.MachinePull` (`self.CondenserTarget`)))
  (bind _output_get (set `self.BoostState` _booldata))
  (for _array_element (`self.BoostStateDisplayTarget`)
    (message `/Game/MachineBlueprints/MachineInterface.DisplayState` _array_element _output_get))
  ;[1 1 1] Set Flow Amount
  (if (and (`self.InputValveState`) (`self.ValveOutState`) (== (`self.WaterInPercent`) 100.0) (`self.PumpState`))
    (set `self.CirculationFlow` (`self.NominalCirculationFlo`)))
  ;[1 1 1] WaterInsideLogic
  (if (and (`self.InputValveState`) (not (`self.ValveOutState`)))
    (bind _output_get_2 (set `self.WaterInPercent` (`KismetMathLibrary.FClamp` (+ (`self.WaterInPercent`) (`self.WaterFillSpeed`)) 0.0 100.0)))
    (elif (and (not (`self.InputValveState`)) (`self.ValveOutState`))
      (set `self.WaterInPercent` (`KismetMathLibrary.FClamp` (- (`self.WaterInPercent`) (`self.WaterFillSpeed`)) 0.0 100.0))))
  (for _array_element_2 (`self.WaterInPercentDisplayTarget`)
    (message `/Game/MachineBlueprints/MachineInterface.DisplayFloat` _array_element_2 _output_get_2)))

(event `self.ReceiveBeginPlay`
  (`self.RefreshDisplay`))

(fn `DisplayState`
  (params (StatePushed :type Boolean))
  (return))

(fn `MachinePull`
  (returns (IntegerData :type Integer) (FloatData :type "Float (double-precision)") (FloatData2 :type "Float (double-precision)") (BoolData :type Boolean) (`Float Data 3` :type "Float (double-precision)") (`Float Data 4` :type "Float (double-precision)"))
  (return 0 (`self.CirculationFlow`) 0.0 false 0.0 0.0))

(fn `RefreshDisplay`
  (for _array_element (`self.ValveInStateDisplayTarget`)
    (message `/Game/MachineBlueprints/MachineInterface.DisplayState` _array_element (`self.InputValveState`)))
  (for _array_element_2 (`self.PumpStateDisplayTarget`)
    (message `/Game/MachineBlueprints/MachineInterface.DisplayState` _array_element_2 (`self.PumpState`)))
  (for _array_element_3 (`self.ValveOutStateDisplayTarget`)
    (message `/Game/MachineBlueprints/MachineInterface.DisplayState` _array_element_3 (`self.ValveOutState`)))
  (for _array_element_4 (`self.BoostStateDisplayTarget`)
    (message `/Game/MachineBlueprints/MachineInterface.DisplayState` _array_element_4 (`self.BoostState`)))
  (for _array_element_5 (`self.WaterInPercentDisplayTarget`)
    (message `/Game/MachineBlueprints/MachineInterface.DisplayFloat` _array_element_5 (`self.WaterInPercent`))))

(fn `UserConstructionScript`)