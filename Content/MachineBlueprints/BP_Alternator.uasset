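; BP_Alternator is a machine Blueprint simulating a turbine-driven alternator that synchronizes with the power grid.
; Each Tick it pulls turbine data, deriving frequency and advancing phase while unlocked, or fixing 3000 RPM/50 Hz and displaying generated power while locked.
; Grid switch input changes the lock only within phase and frequency windows, then notifies the turbine and indicators.
; Its own MachinePull returns only default values.
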(event `/Game/MachineBlueprints/MachineInterface.InputAlternatorGridConnect`
  (params (`Connect to grid` :type Boolean))
  (bind _alternator_frecuency (`self.Alternator Frecuency`))
  (bind _currentgenphase (`self.CurrentGenPhase`))
  ;[1 1 1] Alternator Grid Connection Switch
  (if (and (or (and (>= _currentgenphase 0.0) (<= _currentgenphase (`self.GridConnectMaxDegree`))) (and (<= _currentgenphase 360.0) (>= _currentgenphase (`self.GridConnectMinDegree`)))) (and (>= _alternator_frecuency (`self.GridConnectMinFreq`)) (<= _alternator_frecuency (`self.GridConnectMaxFreq`))))
    (bind _output_get (set `self.AlternatorGridLock` `Connect to grid`))
    (message `/Game/MachineBlueprints/MachineInterface.MachineAlternatorConnectedToGrid` (`self.TurbineTarget`) _output_get :!label _label)
    (for _array_element (`self.AlternatorGridLockIndicatorTargets`)
      (message `/Game/MachineBlueprints/MachineInterface.DisplayState` _array_element _output_get))))

(event `DisplayPush`
  ;[1 1 1] Alternator Grid Connection Switch
  (goto _label))

(event `self.ReceiveBeginPlay`
  (`self.DisplayPush`))

(event `self.ReceiveTick`
  (params (DeltaSeconds :type "Float (single-precision)"))
  (bind _currentgenphase (`self.CurrentGenPhase`))
  ;[1 1 1] Set Alternator RPM
  (bind (_integerdata _floatdata _floatdata2) (message `/Game/MachineBlueprints/MachineInterface.MachinePull` (`self.TurbineTarget`)))
  (if (`self.AlternatorGridLock`)
    ;[1 1 1] If Connected To grid
    (set `self.Alternator RPM` 3000.0)
    (set `self.Alternator Frecuency` 50.0)
    (bind _output_get (set `self.AlternatorElectricalPowerGen` _floatdata2))
    (message `/Game/MachineBlueprints/MachineInterface.DisplayFloat` (`self.PowerGeneratedDisplayTarget`) _output_get)
    (else
      (set `self.AlternatorElectricalPowerGen` 0.0)
      ;[1 1 1] Generator Phase
      (bind _output_get_2 (set `self.Alternator RPM` _floatdata))
      (if (> _output_get_2 0.0)
        (bind _output_get_3 (set `self.Alternator Frecuency` (/ _output_get_2 60.0)))
        (bind _output_get_4 (set `self.CurrentGenPhaseSpeed` (- 18000.0 (* _output_get_3 36.0))))
        (bind _output_get_5 (set `self.CurrentGenPhase` (+ _output_get_4 (`self.CurrentGenPhase`))))
        (if (> _output_get_5 360.0)
          (set `self.CurrentGenPhase` (- _currentgenphase 360.0))
          (elif (< _output_get_5 0.0)
            (set `self.CurrentGenPhase` (+ _currentgenphase 360.0))))))))

(fn `MachinePull`
  (returns (IntegerData :type Integer) (FloatData :type "Float (double-precision)") (FloatData2 :type "Float (double-precision)") (BoolData :type Boolean))
  (return 0 0.0 0.0 false))

(fn `UserConstructionScript`)