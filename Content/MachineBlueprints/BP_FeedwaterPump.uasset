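; Feedwater pump machine that simulates priming and circulation flow from switch and valve inputs.
; A three-way selector steps the main feedwater valve through a repeating Delay loop.
; Tick fills or drains the pump when only the inlet or outlet is open, and scales flow by valve position only when running, full and open at both ends.
; States go to displays via messages, and MachinePull exposes flow.
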(event `/Game/MachineBlueprints/MachineInterface.InputSpeedIntegerSelector`
  (params (ValveStateSelector :type Integer))
  (bind _feedwatervalveselectorspeed (`self.FeedwaterValveSelectorSpeed`))
  ;[1 1 1] CondenserBypassControl
  (if (== ValveStateSelector 0) :!label _label
    (set `self.MainFeedwaterValve` (`KismetMathLibrary.FClamp` (- (`self.MainFeedwaterValve`) _feedwatervalveselectorspeed)))
    (`KismetSystemLibrary.Delay` 0.1 :!label _label_2)
    (goto _label)
    (elif (== ValveStateSelector 2)
      (set `self.MainFeedwaterValve` (`KismetMathLibrary.FClamp` (+ (`self.MainFeedwaterValve`) _feedwatervalveselectorspeed)))
      (goto _label_2))))

(event `self.InputLargePumpValveOut`
  (params (OutValveState :type Boolean))
  (bind _output_get (set `self.ValveOutState` OutValveState))
  (for _array_element (`self.ValveOutStateDisplayTarget`)
    (message `/Game/MachineBlueprints/MachineInterface.DisplayState` _array_element _output_get)))

(event `self.InputLargePumpValveIn`
  (params (InValveState :type Boolean))
  (set `self.InputValveState` InValveState)
  (for _array_element (`self.ValveInStateDisplayTarget`)
    (message `/Game/MachineBlueprints/MachineInterface.DisplayState` _array_element (`self.InputValveState`))))

(event `self.InputStateSwitch`
  (params (State :type Boolean))
  (bind _output_get (set `self.PumpState` State))
  (for _array_element (`self.PumpStateDisplayTarget`)
    (message `/Game/MachineBlueprints/MachineInterface.DisplayState` _array_element _output_get)))

(event `self.ReceiveTick`
  (params (DeltaSeconds :type "Float (single-precision)"))
  ;[1 1 1] Set Flow Amount
  (if (and (`self.InputValveState`) (`self.ValveOutState`) (== (`self.WaterInPercent`) 100.0) (`self.PumpState`))
    (bind _output_get (set `self.CirculationFlow` (`KismetMathLibrary.Lerp` 0.0 (`self.100%CirculationFlow`) (`self.MainFeedwaterValve`))))
    (else
      (set `self.CirculationFlow` 0.0)))
  ;[1 1 1] Speed Display
  (message `/Game/MachineBlueprints/MachineInterface.DisplayFloat` (`self.DisplayFlowTarget`) _output_get)
  ;[1 1 1] WaterInsideLogic
  (if (and (`self.InputValveState`) (not (`self.ValveOutState`)))
    (bind _output_get_2 (set `self.WaterInPercent` (`KismetMathLibrary.FClamp` (+ (`self.WaterInPercent`) (`self.WaterFillSpeed`)) 0.0 100.0)))
    (elif (and (not (`self.InputValveState`)) (`self.ValveOutState`))
      (set `self.WaterInPercent` (`KismetMathLibrary.FClamp` (- (`self.WaterInPercent`) (`self.WaterFillSpeed`)) 0.0 100.0))))
  (for _array_element (`self.WaterInPercentDisplayTarget`)
    (message `/Game/MachineBlueprints/MachineInterface.DisplayFloat` _array_element _output_get_2)))

(event `self.ReceiveBeginPlay`
  (`self.RefreshDisplay`))

(fn `MachinePull`
  (returns (IntegerData :type Integer) (FloatData :type "Float (double-precision)") (FloatData2 :type "Float (double-precision)") (BoolData :type Boolean) (`Float Data 3` :type "Float (double-precision)"))
  (return 0 (`self.CirculationFlow`) 0.0 false 0.0))

(fn `RefreshDisplay`
  (for _array_element (`self.ValveInStateDisplayTarget`)
    (message `/Game/MachineBlueprints/MachineInterface.DisplayState` _array_element (`self.InputValveState`)))
  (for _array_element_2 (`self.PumpStateDisplayTarget`)
    (message `/Game/MachineBlueprints/MachineInterface.DisplayState` _array_element_2 (`self.PumpState`)))
  (for _array_element_3 (`self.ValveOutStateDisplayTarget`)
    (message `/Game/MachineBlueprints/MachineInterface.DisplayState` _array_element_3 (`self.ValveOutState`))
    (for _array_element_4 (`self.WaterInPercentDisplayTarget`)
      (message `/Game/MachineBlueprints/MachineInterface.DisplayFloat` _array_element_4 (`self.WaterInPercent`)))
    (message `/Game/MachineBlueprints/MachineInterface.DisplayFloat` (`self.DisplayFlowTarget`) (* (`self.MainFeedwaterValve`) 100.0))))

(fn `UserConstructionScript`)