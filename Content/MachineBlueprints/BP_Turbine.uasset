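; BP_Turbine simulates a steam turbine machine between a reactor and a condenser.
; Tick derives steam flow from eased reactor pressure and valve opening, exposes it through MachinePull, and converts it to power, calling the trip logic on high condenser pressure.
; RPM is fixed when the alternator is grid-connected, otherwise following stored power with drag.
; Regulator input steps the valve on a delay, and display targets show valve and trip state.
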(event `self.ReceiveBeginPlay`
  (`self.RefreshDisplay`))

(event `TurbineTripEvent`
  ;[1 1 1] Turbine Valve Setting Input
  (if (`self.TurbineTrip`) :!label _label
    (set `self.InputValveState` 0.0)
    (message `/Game/MachineBlueprints/MachineInterface.DisplayFloat` (`self.TurbineValveSettingDisplayTarget`) (* (`self.InputValveState`) 100.0) :!label _label_2)
    (`KismetSystemLibrary.Delay` 0.1)
    (if (== (stale `/Game/MachineBlueprints/MachineInterface.InputTurbineValveRegulator` _output_get) 0) :!label _label_3
      (set `self.InputValveState` (`KismetMathLibrary.FClamp` (- (`self.InputValveState`) (`self.TurbineValveSpeed`))))
      (goto _label_2)
      (elif (== (stale `/Game/MachineBlueprints/MachineInterface.InputTurbineValveRegulator` _output_get) 2)
        (set `self.InputValveState` (`KismetMathLibrary.FClamp` (+ (`self.InputValveState`) (`self.TurbineValveSpeed`))))
        (goto _label_2)))
    (else
      (goto _label_3))))

(event `/Game/MachineBlueprints/MachineInterface.MachineAlternatorConnectedToGrid`
  (params (Connected :type Boolean))
  (set `self.AlternatorState` Connected))

(event `/Game/MachineBlueprints/MachineInterface.InputTurbineValveRegulator`
  (params (TurvineValveSetting :type Integer))
  ;[1 1 1] Turbine Valve Setting Input
  (bind _output_get (set `self.TurbienValveSetting` TurvineValveSetting))
  (goto _label))

(event `/Game/MachineBlueprints/MachineInterface.InputTurbineEnable`
  (params (`Trip status` :type Boolean))
  (bind _output_get (set `self.TurbineTrip` `Trip status`))
  (for _array_element (`self.TurbineTripDisplayTargets`)
    (message `/Game/MachineBlueprints/MachineInterface.DisplayState` _array_element _output_get)))

(event `self.ReceiveTick`
  (params (DeltaSeconds :type "Float (single-precision)"))
  (bind _powerstored (`self.PowerStored`))
  ;[1 1 1] Find Steam Input
  (if (`self.TurbineTrip`)
    (bind (_integerdata _floatdata) (message `/Game/MachineBlueprints/MachineInterface.MachinePull` (`self.ReactorTarget`)))
    (bind _output_get (set `self.ReactorPressurekPa` _floatdata))
    (bind _output_get_2 (set `self.SteamInKg` (* (`|EaseFunction` "EaseIn" (/ _output_get (`self.ReactorNominalPressure`)) 0.0 (`self.ReactorNominal100KgIn`)) (`self.InputValveState`))))
    ;[1 1 1] Distribute Steam
    (set `self.SteamOut` _output_get_2)
    ;[1 1 1] Set Power Generated
    (bind (_integerdata_2 _floatdata_2) (message `/Game/MachineBlueprints/MachineInterface.MachinePull` (`self.CondenserTarget`)))
    (bind _output_get_3 (set `self.CondenserPressure` _floatdata_2))
    (if (<= _output_get_3 (`self.TurbineCondenserHighPressureTrip`))
      (set `self.PowerProduced` (`KismetMathLibrary.Lerp` 0.0 (`self.Powerat100Nominal`) (/ (`self.SteamInKg`) (`self.ReactorNominal100KgIn`))))
      ;[1 1 1] Turbine Speed Calculation
      (if (`self.AlternatorState`) :!label _label_4
        (set `self.TurbineRPM` 3000.0)
        (else
          (bind _output_get_4 (set `self.PowerStored` (`KismetMathLibrary.FClamp` (- (+ (`self.PowerProduced`) _powerstored) (* _powerstored (`self.DragMultiplier`))) 0.0 100000.0)))
          (set `self.TurbineRPM` (`KismetMathLibrary.Lerp` 0.0 3000.0 (/ _output_get_4 (`self.PowerStoredAt3000`))))))
      (else
        (`self.InputTurbineEnable` true)
        (`self.TurbineTripEvent`)))
    (else
      (goto _label_4))))

(fn `MachinePull`
  (returns (IntegerData :type Integer) (FloatData :type "Float (double-precision)") (FloatData2 :type "Float (double-precision)") (BoolData :type Boolean))
  (return 0 (`self.SteamOut`) 0.0 false))

(fn `RefreshDisplay`
  (for _array_element (`self.TurbineTripDisplayTargets`)
    (message `/Game/MachineBlueprints/MachineInterface.DisplayState` _array_element (`self.TurbineTrip`)))
  (message `/Game/MachineBlueprints/MachineInterface.DisplayFloat` (`self.TurbineValveSettingDisplayTarget`) (`self.InputValveState`)))

(fn `UserConstructionScript`)