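; Reactor circulation pump machine that simulates water fill and circulation flow from valve, switch and speed inputs.
; Input events store valve and pump states, while the speed selector steps PumpSpeed in a delayed loop, clamped only when increasing.
; Tick fills or drains water by valve combination and sets flow from speed when full, open and on, never resetting it otherwise.
; States and readings are pushed to display target arrays.
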(event `/Game/MachineBlueprints/MachineInterface.InputSpeedIntegerSelector`
  (params (ValveStateSelector :type Integer))
  (if (== ValveStateSelector 2) :!label _label
    (bind _output_get (set `self.PumpSpeed` (`KismetMathLibrary.FClamp` (+ (`self.PumpSpeed`) (`self.PumpSpeedSettingSpeed`)) 0.0 1.0)))
    (for _array_element (`self.PumpSpeedDisplayTargets`) :!label _label_2
      (message `/Game/MachineBlueprints/MachineInterface.DisplayFloat` _array_element _output_get))
    (`KismetSystemLibrary.Delay` 0.1)
    (goto _label)
    (elif (== ValveStateSelector 0)
      (set `self.PumpSpeed` (- (`self.PumpSpeed`) (`self.PumpSpeedSettingSpeed`)))
      (goto _label_2))))

(event `/Game/MachineBlueprints/MachineInterface.InputLargePumpValveOut`
  (params (OutValveState :type Boolean))
  (bind _output_get (set `self.ValveOutState` OutValveState))
  (for _array_element (`self.ValveOutDisplayTarget`)
    (message `/Game/MachineBlueprints/MachineInterface.DisplayState` _array_element _output_get)))

(event `/Game/MachineBlueprints/MachineInterface.InputLargePumpValveIn`
  (params (InValveState :type Boolean))
  (bind _output_get (set `self.InputValveState` InValveState))
  (for _array_element (`self.ValveInDisplayTarget`)
    (message `/Game/MachineBlueprints/MachineInterface.DisplayState` _array_element _output_get)))

(event `/Game/MachineBlueprints/MachineInterface.InputStateSwitch`
  (params (State :type Boolean))
  (bind _output_get (set `self.PumpState` State))
  (for _array_element (`self.Pump State Display Target`)
    (message `/Game/MachineBlueprints/MachineInterface.DisplayState` _array_element _output_get)))

(event `self.ReceiveTick`
  (params (DeltaSeconds :type "Float (single-precision)"))
  ;[1 1 1] Set Flow Amount
  (if (and (`self.InputValveState`) (`self.ValveOutState`) (== (`self.WaterInPercent`) 100.0) (`self.PumpState`))
    (set `self.CirculationFlow` (* (`self.NominalCirculationFlow`) (`self.PumpSpeed`))))
  ;[1 1 1] WaterInsideLogic
  (if (and (`self.InputValveState`) (not (`self.ValveOutState`)))
    (bind _output_get (set `self.WaterInPercent` (`KismetMathLibrary.FClamp` (+ (`self.WaterInPercent`) (`self.WaterFillSpeed`)) 0.0 100.0)))
    (elif (and (not (`self.InputValveState`)) (`self.ValveOutState`))
      (set `self.WaterInPercent` (`KismetMathLibrary.FClamp` (- (`self.WaterInPercent`) (`self.WaterFillSpeed`)) 0.0 100.0))))
  (for _array_element (`self.WaterInPercentDisplayTarget`)
    (message `/Game/MachineBlueprints/MachineInterface.DisplayDoubleFloat` _array_element (`self.CirculationFlow`) _output_get)))

(event `self.ReceiveBeginPlay`
  (`self.RefreshDisplay`))

(fn `MachinePull`
  (returns (IntegerData :type Integer) (FloatData :type "Float (double-precision)") (FloatData2 :type "Float (double-precision)") (BoolData :type Boolean) (`Float Data 3` :type "Float (double-precision)"))
  (return 0 0.0 0.0 false 0.0))

(fn `RefreshDisplay`
  (for _array_element (`self.Pump State Display Target`)
    (message `/Game/MachineBlueprints/MachineInterface.DisplayState` _array_element (`self.PumpState`)))
  (for _array_element_2 (`self.ValveInDisplayTarget`)
    (message `/Game/MachineBlueprints/MachineInterface.DisplayState` _array_element_2 (`self.InputValveState`)))
  (for _array_element_3 (`self.ValveOutDisplayTarget`)
    (message `/Game/MachineBlueprints/MachineInterface.DisplayState` _array_element_3 (`self.ValveOutState`)))
  (for _array_element_4 (`self.WaterInpercentDisplayTarget`)
    (message `/Game/MachineBlueprints/MachineInterface.DisplayFloat` _array_element_4 (`self.WaterInPercent`)))
  (for _array_element_5 (`self.PumpSpeedDisplayTargets`)
    (message `/Game/MachineBlueprints/MachineInterface.DisplayFloat` _array_element_5 (`self.PumpSpeed`))))

(fn `UserConstructionScript`)