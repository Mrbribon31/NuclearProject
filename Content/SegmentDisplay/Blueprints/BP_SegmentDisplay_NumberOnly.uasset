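; BP_SegmentDisplay_NumberOnly is a segment display variant that shows an integer.
; UpdateNumber converts Number to ungrouped text padded to at least Length digits, stores the string in Value and calls Update to refresh the display.
; It runs from the Construction Script, after the parent's script, and again on BeginPlay.
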(event `self.ReceiveBeginPlay`
  (`self.UpdateNumber`))

(fn `UpdateNumber`
  ;[1 1 1] Updates display value using number
  (set `self.Value` (`KismetTextLibrary.Conv_TextToString` (`KismetTextLibrary.Conv_IntToText` (`self.Number`) false false (`self.Length`))))
  (`self.Update`))

(fn `UserConstructionScript`
  (`parent.UserConstructionScript`)
  (`self.UpdateNumber`))