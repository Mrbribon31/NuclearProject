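; Segment display Blueprint that acts as a clock or countdown, showing zero-padded hours, minutes and seconds.
; With RealTimeUpdate on, a looping timer of SecondTime length ticks the time forward, or backward if Reverse is set, rolling over on a 24-hour cycle.
; In Countdown mode, a reverse rollover past zero pauses the timer and calls CountdownAtZero, a placeholder that prints a message.
; UpdateTime formats the display string at construction and on ticks.
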(event `self.ReceiveBeginPlay`
  (`self.UpdateTime`)
  (if (`self.bRealTimeUpdate`)
    ;[1 1 1] How long a Second lasts is handled here
    (bind _returnvalue (`KismetSystemLibrary.K2_SetTimerDelegate` (`|CreateDelegate` :!event `UpdateSecond`) (`self.SecondTime`) true))
    (set `self.UpdateSecond_Handle` _returnvalue)))

(event `UpdateSecond`
  ;[1 1 1] Updates display every minute and handles logic for display values
  (if (`self.bReverse`)
    (if (<= (`self.Second`) 0)
      (set `self.Second` 59)
      (if (<= (`self.Minute`) 0)
        (set `self.Minute` 59)
        (if (<= (`self.Hour`) 0)
          (if (`self.bCountdown`)
            (`KismetSystemLibrary.K2_PauseTimerHandle` (`self.UpdateSecond_Handle`))
            (`self.CountdownAtZero`)
            (else
              (set `self.Hour` 23)
              (`self.UpdateTime` :!label _label)))
          (else
            (`/Engine/EditorBlueprintResources/StandardMacros.DecrementInt` (`self.Hour`)
              (:`  `
                (goto _label)))))
        (else
          (`/Engine/EditorBlueprintResources/StandardMacros.DecrementInt` (`self.Minute`)
            (:`  `
              (goto _label)))))
      (else
        (`/Engine/EditorBlueprintResources/StandardMacros.DecrementInt` (`self.Second`)
          (:`  `
            (goto _label)))))
    (else
      (if (>= (`self.Second`) 59)
        (set `self.Second` 0)
        (if (>= (`self.Minute`) 59)
          (set `self.Minute` 0)
          (if (>= (`self.Hour`) 23)
            (set `self.Hour` 0)
            (else
              (`/Engine/EditorBlueprintResources/StandardMacros.IncrementInt` (`self.Hour`)
                (:`  `
                  _))))
          (else
            (`/Engine/EditorBlueprintResources/StandardMacros.IncrementInt` (`self.Minute`)
              (:`  `
                _))))
        (else
          (`/Engine/EditorBlueprintResources/StandardMacros.IncrementInt` (`self.Second`)
            (:`  `
              _))))
      (`self.UpdateTime`))))

(event `CountdownAtZero`
  ;[1 1 1] Add your own function here when timer reaches zero (Event dispatch, call actor)
  (`KismetSystemLibrary.PrintString` "Countdown at zero" true true (struct :`R` 1.0 :`G` 0.080507 :`A` 1.0)))

(fn `UpdateTime`
  ;[1 1 1] Sets display value using hour and minute values
  (set `self.Value` (`KismetTextLibrary.Conv_TextToString` (`|FormatText` "{Hour}:{Minute}:{Second}" (`KismetTextLibrary.Conv_IntToText` (`self.Hour`) false true 2 2) (`KismetTextLibrary.Conv_IntToText` (`self.Minute`) false true 2 2) (`KismetTextLibrary.Conv_IntToText` (`self.Second`) false true 2 2))))
  (`self.Update`))

(fn `UserConstructionScript`
  (`parent.UserConstructionScript`)
  (`self.UpdateTime`))