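; Segment display actor that shows a text string on a row of 7-segment, 16-segment or matrix style character meshes.
; The construction script spawns Length evenly spaced meshes with the chosen material, then applies brightness, colour, background opacity and on/off parameters.
; Each character of Value sets Column and Row parameters to pick its material atlas glyph.
; UpdateValue and TurnOnOff refresh existing segments without rebuilding; segments past the string's end stay unchanged.
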(fn `Construct Core`
  ;[1 1 1] Generates mesh array and applys settings then adds material
  (`self.SetLength`)
  (for _array_element (`self.SegmentArray`)
    (`StaticMeshComponent.SetStaticMesh` _array_element "/Game/SegmentDisplay/Meshes/SM_Display_Segment.SM_Display_Segment") ; Add custom mesh here
    (`PrimitiveComponent.SetCastShadow` _array_element false) ; Disable shadows makes it look better
    (`self.SetSegmentType` _array_element)))

(fn `Construct Update`
  ;[1 1 1] Applys material settings and updates display value
  (for _array_element (`self.SegmentArray`)
    (`self.Material Settings` _array_element))
  (`self.Update`))

(fn `Material Settings`
  (params (Mesh :type "MeshComponent Object Reference"))
  ;[1 1 1] Modifies material settings
  (`MeshComponent.SetScalarParameterValueOnMaterials` Mesh "Emmissive Strength" (`KismetMathLibrary.SelectFloat` (`self.Brightness`) 0.0 (`self.bOn`)))
  (`MeshComponent.SetVectorParameterValueOnMaterials` Mesh "Colour" (`KismetMathLibrary.Conv_LinearColorToVector` (`self.Colour`)))
  (`MeshComponent.SetScalarParameterValueOnMaterials` Mesh "Background Opacity" (`self.Background Opacity`))
  (`MeshComponent.SetScalarParameterValueOnMaterials` Mesh "OffSwitch" (`KismetMathLibrary.SelectFloat` 0.0 1.0 (`self.bOn`))))

(fn `SetDisplayValue`
  (params (Mesh :type "MeshComponent Object Reference") (Value :type String))
  ;[1 1 1] Takes each character and chooses correct material atlas position
  ;;[1 1 1] Check if space
  (if (`KismetStringLibrary.EqualEqual_StrStr` Value " ")
    ;[1 1 1] Space
    (`MeshComponent.SetScalarParameterValueOnMaterials` Mesh "Column" 8.0)
    (`MeshComponent.SetScalarParameterValueOnMaterials` Mesh "Row" 8.0)
    (else
      ;;[1 1 1] Checks if character is uppercase
      (if (`KismetStringLibrary.EqualEqual_StrStr` Value (`KismetStringLibrary.ToUpper` Value))
        (switch `string` Value
          (:`0`
            ;[1 1 1] 0 - 9
            (`MeshComponent.SetScalarParameterValueOnMaterials` Mesh "Column" 0.0)
            (`MeshComponent.SetScalarParameterValueOnMaterials` Mesh "Row" 0.0))
          (:`1`
            (`MeshComponent.SetScalarParameterValueOnMaterials` Mesh "Column" 0.0)
            (`MeshComponent.SetScalarParameterValueOnMaterials` Mesh "Row" 1.0))
          (:`2`
            (`MeshComponent.SetScalarParameterValueOnMaterials` Mesh "Column" 0.0)
            (`MeshComponent.SetScalarParameterValueOnMaterials` Mesh "Row" 2.0))
          (:`3`
            (`MeshComponent.SetScalarParameterValueOnMaterials` Mesh "Column" 0.0)
            (`MeshComponent.SetScalarParameterValueOnMaterials` Mesh "Row" 3.0))
          (:`4`
            (`MeshComponent.SetScalarParameterValueOnMaterials` Mesh "Column" 0.0)
            (`MeshComponent.SetScalarParameterValueOnMaterials` Mesh "Row" 4.0))
          (:`5`
            (`MeshComponent.SetScalarParameterValueOnMaterials` Mesh "Column" 0.0)
            (`MeshComponent.SetScalarParameterValueOnMaterials` Mesh "Row" 5.0))
          (:`6`
            (`MeshComponent.SetScalarParameterValueOnMaterials` Mesh "Column" 0.0)
            (`MeshComponent.SetScalarParameterValueOnMaterials` Mesh "Row" 6.0))
          (:`7`
            (`MeshComponent.SetScalarParameterValueOnMaterials` Mesh "Column" 0.0)
            (`MeshComponent.SetScalarParameterValueOnMaterials` Mesh "Row" 7.0))
          (:`8`
            (`MeshComponent.SetScalarParameterValueOnMaterials` Mesh "Column" 0.0)
            (`MeshComponent.SetScalarParameterValueOnMaterials` Mesh "Row" 8.0))
          (:`9`
            (`MeshComponent.SetScalarParameterValueOnMaterials` Mesh "Column" 1.0)
            (`MeshComponent.SetScalarParameterValueOnMaterials` Mesh "Row" 0.0))
          (:`A`
            ;[1 1 1] Letters Uppercase
            (`MeshComponent.SetScalarParameterValueOnMaterials` Mesh "Column" 1.0)
            (`MeshComponent.SetScalarParameterValueOnMaterials` Mesh "Row" 1.0))
          (:`B`
            (`MeshComponent.SetScalarParameterValueOnMaterials` Mesh "Column" 1.0)
            (`MeshComponent.SetScalarParameterValueOnMaterials` Mesh "Row" 2.0))
          (:`C`
            (`MeshComponent.SetScalarParameterValueOnMaterials` Mesh "Column" 1.0)
            (`MeshComponent.SetScalarParameterValueOnMaterials` Mesh "Row" 3.0))
          (:`D`
            (`MeshComponent.SetScalarParameterValueOnMaterials` Mesh "Column" 1.0)
            (`MeshComponent.SetScalarParameterValueOnMaterials` Mesh "Row" 4.0))
          (:`E`
            (`MeshComponent.SetScalarParameterValueOnMaterials` Mesh "Column" 1.0)
            (`MeshComponent.SetScalarParameterValueOnMaterials` Mesh "Row" 5.0))
          (:`F`
            (`MeshComponent.SetScalarParameterValueOnMaterials` Mesh "Column" 1.0)
            (`MeshComponent.SetScalarParameterValueOnMaterials` Mesh "Row" 6.0))
          (:`G`
            (`MeshComponent.SetScalarParameterValueOnMaterials` Mesh "Column" 1.0)
            (`MeshComponent.SetScalarParameterValueOnMaterials` Mesh "Row" 7.0))
          (:`H`
            (`MeshComponent.SetScalarParameterValueOnMaterials` Mesh "Column" 1.0)
            (`MeshComponent.SetScalarParameterValueOnMaterials` Mesh "Row" 8.0))
          (:`I`
            (`MeshComponent.SetScalarParameterValueOnMaterials` Mesh "Column" 2.0)
            (`MeshComponent.SetScalarParameterValueOnMaterials` Mesh "Row" 0.0))
          (:`J`
            (`MeshComponent.SetScalarParameterValueOnMaterials` Mesh "Column" 2.0)
            (`MeshComponent.SetScalarParameterValueOnMaterials` Mesh "Row" 1.0))
          (:`K`
            (`MeshComponent.SetScalarParameterValueOnMaterials` Mesh "Column" 2.0)
            (`MeshComponent.SetScalarParameterValueOnMaterials` Mesh "Row" 2.0))
          (:`L`
            (`MeshComponent.SetScalarParameterValueOnMaterials` Mesh "Column" 2.0)
            (`MeshComponent.SetScalarParameterValueOnMaterials` Mesh "Row" 3.0))
          (:`M`
            (`MeshComponent.SetScalarParameterValueOnMaterials` Mesh "Column" 2.0)
            (`MeshComponent.SetScalarParameterValueOnMaterials` Mesh "Row" 4.0))
          (:`N`
            (`MeshComponent.SetScalarParameterValueOnMaterials` Mesh "Column" 2.0)
            (`MeshComponent.SetScalarParameterValueOnMaterials` Mesh "Row" 5.0))
          (:`O`
            (`MeshComponent.SetScalarParameterValueOnMaterials` Mesh "Column" 2.0)
            (`MeshComponent.SetScalarParameterValueOnMaterials` Mesh "Row" 6.0))
          (:`P`
            (`MeshComponent.SetScalarParameterValueOnMaterials` Mesh "Column" 2.0)
            (`MeshComponent.SetScalarParameterValueOnMaterials` Mesh "Row" 7.0))
          (:`Q`
            (`MeshComponent.SetScalarParameterValueOnMaterials` Mesh "Column" 2.0)
            (`MeshComponent.SetScalarParameterValueOnMaterials` Mesh "Row" 8.0))
          (:`R`
            (`MeshComponent.SetScalarParameterValueOnMaterials` Mesh "Column" 3.0)
            (`MeshComponent.SetScalarParameterValueOnMaterials` Mesh "Row" 0.0))
          (:`S`
            (`MeshComponent.SetScalarParameterValueOnMaterials` Mesh "Column" 3.0)
            (`MeshComponent.SetScalarParameterValueOnMaterials` Mesh "Row" 1.0))
          (:`T`
            (`MeshComponent.SetScalarParameterValueOnMaterials` Mesh "Column" 3.0)
            (`MeshComponent.SetScalarParameterValueOnMaterials` Mesh "Row" 2.0))
          (:`U`
            (`MeshComponent.SetScalarParameterValueOnMaterials` Mesh "Column" 3.0)
            (`MeshComponent.SetScalarParameterValueOnMaterials` Mesh "Row" 3.0))
          (:`V`
            (`MeshComponent.SetScalarParameterValueOnMaterials` Mesh "Column" 3.0)
            (`MeshComponent.SetScalarParameterValueOnMaterials` Mesh "Row" 4.0))
          (:`W`
            (`MeshComponent.SetScalarParameterValueOnMaterials` Mesh "Column" 3.0)
            (`MeshComponent.SetScalarParameterValueOnMaterials` Mesh "Row" 5.0))
          (:`X`
            (`MeshComponent.SetScalarParameterValueOnMaterials` Mesh "Column" 3.0)
            (`MeshComponent.SetScalarParameterValueOnMaterials` Mesh "Row" 6.0))
          (:`Y`
            (`MeshComponent.SetScalarParameterValueOnMaterials` Mesh "Column" 3.0)
            (`MeshComponent.SetScalarParameterValueOnMaterials` Mesh "Row" 7.0))
          (:`Z`
            (`MeshComponent.SetScalarParameterValueOnMaterials` Mesh "Column" 3.0)
            (`MeshComponent.SetScalarParameterValueOnMaterials` Mesh "Row" 8.0))
          (:`:`
            ;[1 1 1] Symbols
            (`MeshComponent.SetScalarParameterValueOnMaterials` Mesh "Column" 6.0)
            (`MeshComponent.SetScalarParameterValueOnMaterials` Mesh "Row" 8.0))
          (:`^`
            (`MeshComponent.SetScalarParameterValueOnMaterials` Mesh "Column" 7.0)
            (`MeshComponent.SetScalarParameterValueOnMaterials` Mesh "Row" 0.0))
          (:`/`
            (`MeshComponent.SetScalarParameterValueOnMaterials` Mesh "Column" 7.0)
            (`MeshComponent.SetScalarParameterValueOnMaterials` Mesh "Row" 1.0))
          (:`[`
            (`MeshComponent.SetScalarParameterValueOnMaterials` Mesh "Column" 7.0)
            (`MeshComponent.SetScalarParameterValueOnMaterials` Mesh "Row" 2.0))
          (:`]`
            (`MeshComponent.SetScalarParameterValueOnMaterials` Mesh "Column" 7.0)
            (`MeshComponent.SetScalarParameterValueOnMaterials` Mesh "Row" 3.0))
          (:`=`
            (`MeshComponent.SetScalarParameterValueOnMaterials` Mesh "Column" 7.0)
            (`MeshComponent.SetScalarParameterValueOnMaterials` Mesh "Row" 4.0))
          (:`+`
            (`MeshComponent.SetScalarParameterValueOnMaterials` Mesh "Column" 7.0)
            (`MeshComponent.SetScalarParameterValueOnMaterials` Mesh "Row" 5.0))
          (:`-`
            (`MeshComponent.SetScalarParameterValueOnMaterials` Mesh "Column" 7.0)
            (`MeshComponent.SetScalarParameterValueOnMaterials` Mesh "Row" 6.0))
          (:`!`
            (`MeshComponent.SetScalarParameterValueOnMaterials` Mesh "Column" 7.0)
            (`MeshComponent.SetScalarParameterValueOnMaterials` Mesh "Row" 7.0))
          (:`£`
            (`MeshComponent.SetScalarParameterValueOnMaterials` Mesh "Column" 7.0)
            (`MeshComponent.SetScalarParameterValueOnMaterials` Mesh "Row" 8.0))
          (:`$`
            (`MeshComponent.SetScalarParameterValueOnMaterials` Mesh "Column" 8.0)
            (`MeshComponent.SetScalarParameterValueOnMaterials` Mesh "Row" 0.0))
          (:`?`
            (`MeshComponent.SetScalarParameterValueOnMaterials` Mesh "Column" 8.0)
            (`MeshComponent.SetScalarParameterValueOnMaterials` Mesh "Row" 1.0)))
        (else
          (switch `string` Value
            (:`A`
              ;[1 1 1] Letters Lowercase
              (`MeshComponent.SetScalarParameterValueOnMaterials` Mesh "Column" 4.0)
              (`MeshComponent.SetScalarParameterValueOnMaterials` Mesh "Row" 0.0))
            (:`B`
              (`MeshComponent.SetScalarParameterValueOnMaterials` Mesh "Column" 4.0)
              (`MeshComponent.SetScalarParameterValueOnMaterials` Mesh "Row" 1.0))
            (:`C`
              (`MeshComponent.SetScalarParameterValueOnMaterials` Mesh "Column" 4.0)
              (`MeshComponent.SetScalarParameterValueOnMaterials` Mesh "Row" 2.0))
            (:`D`
              (`MeshComponent.SetScalarParameterValueOnMaterials` Mesh "Column" 4.0)
              (`MeshComponent.SetScalarParameterValueOnMaterials` Mesh "Row" 3.0))
            (:`E`
              (`MeshComponent.SetScalarParameterValueOnMaterials` Mesh "Column" 4.0)
              (`MeshComponent.SetScalarParameterValueOnMaterials` Mesh "Row" 4.0))
            (:`F`
              (`MeshComponent.SetScalarParameterValueOnMaterials` Mesh "Column" 4.0)
              (`MeshComponent.SetScalarParameterValueOnMaterials` Mesh "Row" 5.0))
            (:`G`
              (`MeshComponent.SetScalarParameterValueOnMaterials` Mesh "Column" 4.0)
              (`MeshComponent.SetScalarParameterValueOnMaterials` Mesh "Row" 6.0))
            (:`H`
              (`MeshComponent.SetScalarParameterValueOnMaterials` Mesh "Column" 4.0)
              (`MeshComponent.SetScalarParameterValueOnMaterials` Mesh "Row" 7.0))
            (:`i`
              (`MeshComponent.SetScalarParameterValueOnMaterials` Mesh "Column" 4.0)
              (`MeshComponent.SetScalarParameterValueOnMaterials` Mesh "Row" 8.0))
            (:`j`
              (`MeshComponent.SetScalarParameterValueOnMaterials` Mesh "Column" 5.0)
              (`MeshComponent.SetScalarParameterValueOnMaterials` Mesh "Row" 0.0))
            (:`k`
              (`MeshComponent.SetScalarParameterValueOnMaterials` Mesh "Column" 5.0)
              (`MeshComponent.SetScalarParameterValueOnMaterials` Mesh "Row" 1.0))
            (:`l`
              (`MeshComponent.SetScalarParameterValueOnMaterials` Mesh "Column" 5.0)
              (`MeshComponent.SetScalarParameterValueOnMaterials` Mesh "Row" 2.0))
            (:`m`
              (`MeshComponent.SetScalarParameterValueOnMaterials` Mesh "Column" 5.0)
              (`MeshComponent.SetScalarParameterValueOnMaterials` Mesh "Row" 3.0))
            (:`n`
              (`MeshComponent.SetScalarParameterValueOnMaterials` Mesh "Column" 5.0)
              (`MeshComponent.SetScalarParameterValueOnMaterials` Mesh "Row" 4.0))
            (:`o`
              (`MeshComponent.SetScalarParameterValueOnMaterials` Mesh "Column" 5.0)
              (`MeshComponent.SetScalarParameterValueOnMaterials` Mesh "Row" 5.0))
            (:`p`
              (`MeshComponent.SetScalarParameterValueOnMaterials` Mesh "Column" 5.0)
              (`MeshComponent.SetScalarParameterValueOnMaterials` Mesh "Row" 6.0))
            (:`q`
              (`MeshComponent.SetScalarParameterValueOnMaterials` Mesh "Column" 5.0)
              (`MeshComponent.SetScalarParameterValueOnMaterials` Mesh "Row" 7.0))
            (:`r`
              (`MeshComponent.SetScalarParameterValueOnMaterials` Mesh "Column" 5.0)
              (`MeshComponent.SetScalarParameterValueOnMaterials` Mesh "Row" 8.0))
            (:`s`
              (`MeshComponent.SetScalarParameterValueOnMaterials` Mesh "Column" 6.0)
              (`MeshComponent.SetScalarParameterValueOnMaterials` Mesh "Row" 0.0))
            (:`t`
              (`MeshComponent.SetScalarParameterValueOnMaterials` Mesh "Column" 6.0)
              (`MeshComponent.SetScalarParameterValueOnMaterials` Mesh "Row" 1.0))
            (:`u`
              (`MeshComponent.SetScalarParameterValueOnMaterials` Mesh "Column" 6.0)
              (`MeshComponent.SetScalarParameterValueOnMaterials` Mesh "Row" 2.0))
            (:`v`
              (`MeshComponent.SetScalarParameterValueOnMaterials` Mesh "Column" 6.0)
              (`MeshComponent.SetScalarParameterValueOnMaterials` Mesh "Row" 3.0))
            (:`w`
              (`MeshComponent.SetScalarParameterValueOnMaterials` Mesh "Column" 6.0)
              (`MeshComponent.SetScalarParameterValueOnMaterials` Mesh "Row" 4.0))
            (:`x`
              (`MeshComponent.SetScalarParameterValueOnMaterials` Mesh "Column" 6.0)
              (`MeshComponent.SetScalarParameterValueOnMaterials` Mesh "Row" 5.0))
            (:`y`
              (`MeshComponent.SetScalarParameterValueOnMaterials` Mesh "Column" 6.0)
              (`MeshComponent.SetScalarParameterValueOnMaterials` Mesh "Row" 6.0))
            (:`z`
              (`MeshComponent.SetScalarParameterValueOnMaterials` Mesh "Column" 6.0)
              (`MeshComponent.SetScalarParameterValueOnMaterials` Mesh "Row" 7.0))))))))

(fn `SetLength`
  ;[1 1 1] Takes value "Length" and uses to add static meshes to the blueprint
  (for _index (range (`self.Length`))
    (bind _returnvalue (`AddComponent|NODE_AddStaticMeshComponent-1` :`RelativeTransform` (`KismetMathLibrary.MakeTransform` (`KismetMathLibrary.MakeVector` (* _index (`self.Distance`))))))
    (`KismetArrayLibrary.Array_Add` (`self.SegmentArray`) _returnvalue)))

(fn `SetSegmentType`
  (params (Mesh :type "PrimitiveComponent Object Reference"))
  ;[1 1 1] Uses Enum to select the material used
  (switch `/Game/SegmentDisplay/Blueprints/Assets/Enum_SegmentDisplayType` (`self.Segment Type`)
    (:`NewEnumerator0`
      (`PrimitiveComponent.SetMaterial` Mesh 0 "/Game/SegmentDisplay/Materials/Instances/MI_07_Segment_A.MI_07_Segment_A"))
    (:`NewEnumerator12`
      (`PrimitiveComponent.SetMaterial` Mesh 0 "/Game/SegmentDisplay/Materials/Instances/MI_07_Segment_B.MI_07_Segment_B"))
    (:`NewEnumerator1`
      (`PrimitiveComponent.SetMaterial` Mesh 0 "/Game/SegmentDisplay/Materials/Instances/MI_16_Segment_A.MI_16_Segment_A"))
    (:`NewEnumerator13`
      (`PrimitiveComponent.SetMaterial` Mesh 0 "/Game/SegmentDisplay/Materials/Instances/MI_16_Segment_B.MI_16_Segment_B"))
    (:`NewEnumerator2`
      (`PrimitiveComponent.SetMaterial` Mesh 0 "/Game/SegmentDisplay/Materials/Instances/MI_Matrix_Connected_A.MI_Matrix_Connected_A"))
    (:`NewEnumerator8`
      (`PrimitiveComponent.SetMaterial` Mesh 0 "/Game/SegmentDisplay/Materials/Instances/MI_Matrix_Connected_B.MI_Matrix_Connected_B"))
    (:`NewEnumerator9`
      (`PrimitiveComponent.SetMaterial` Mesh 0 "/Game/SegmentDisplay/Materials/Instances/MI_Matrix_Connected_C.MI_Matrix_Connected_C"))
    (:`NewEnumerator3`
      (`PrimitiveComponent.SetMaterial` Mesh 0 "/Game/SegmentDisplay/Materials/Instances/MI_Matrix_Seperated_A.MI_Matrix_Seperated_A"))
    (:`NewEnumerator10`
      (`PrimitiveComponent.SetMaterial` Mesh 0 "/Game/SegmentDisplay/Materials/Instances/MI_Matrix_Seperated_B.MI_Matrix_Seperated_B"))
    (:`NewEnumerator11`
      (`PrimitiveComponent.SetMaterial` Mesh 0 "/Game/SegmentDisplay/Materials/Instances/MI_Matrix_Seperated_C.MI_Matrix_Seperated_C"))))

(fn `TurnOn/Off`
  (params (bOn :type Boolean))
  (set `self.bOn` bOn)
  (for _array_element (`self.SegmentArray`)
    (`self.Material Settings` _array_element)))

(fn `Update`
  (bind _returnvalue (`KismetStringLibrary.GetCharacterArrayFromString` (`self.Value`)))
  ;[1 1 1] Runs though each segment in the array and updates the displayed value
  (for (_array_element _array_index) (`self.SegmentArray`)
    (if (>= _array_index (`KismetArrayLibrary.Array_Length` _returnvalue))
      (break)
      (else
        (`self.SetDisplayValue` _array_element (`|GetArrayItem` _returnvalue _array_index))))))

(fn `UpdateValue`
  (params (Value :type String))
  (set `self.Value` Value)
  (`self.Update`))

(fn `UserConstructionScript`
  ;[1 1 1] Core setup (Expensive)
  (`self.Construct Core`)
  ;[1 1 1] Core update (Not as expensive) If you want to update settings in real time run this
  (`self.Construct Update`))