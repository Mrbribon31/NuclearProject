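; BP_KnobSpeedSelector is an interactable rotary knob that selects a discrete speed setting by mouse drag.
; BeginPlay builds evenly spaced normalized setpoints from the switch count and poses the arrow at the current one.
; Holding adds mouse input to the rotation within soft limits, lerped to arrow roll.
; Releasing snaps to a setpoint within tolerance and sends its index to InteractionTarget, otherwise reverts to the previous position.
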(event `self.ReceiveBeginPlay`
  (bind _arrow (`self.Arrow`))
  (bind _switch_amount (`self.Switch Amount`))
  (bind _arrayindexselector (`self.ArrayIndexSelector`))
  (bind _output (`|GetArrayItem` (`self.Setpoints`) (`self.SwitchValue`)))
  (bind (_relativerotation_roll _relativerotation_pitch _relativerotation_yaw) (`KismetMathLibrary.BreakRotator` (`SceneComponent.RelativeRotation` _arrow)))
  ;[1 1 1] Rotation Snap Points Calculation
  (bind _output_get (set `self.SetpointSpacing` (/ 1.0 (`KismetMathLibrary.Conv_IntToDouble` (- _switch_amount 1)))))
  (set `self.Setpoint Sensitivity` (* (/ _output_get 2.0) (`self.SetpointRange`)))
  (while (not (== _arrayindexselector _switch_amount))
    (`KismetArrayLibrary.Array_Set` (`self.Setpoints`) _arrayindexselector (`self.SetpointSpacingLoop`) true)
    (set `self.SetpointSpacingLoop` (+ (`self.SetpointSpacingLoop`) (`self.SetpointSpacing`)))
    (set `self.ArrayIndexSelector` (+ _arrayindexselector 1)))
  (bind _location (`self.Parameterize Position` _output :!label _label))
  (`SceneComponent.K2_SetRelativeRotation` _arrow (`KismetMathLibrary.MakeRotator` _location _relativerotation_pitch _relativerotation_yaw) false false)
  (set `self.CurrentRotation` _output))

(event `self.HoldInteractStop`
  (bind _arrow (`self.Arrow`))
  (bind (_relativerotation_roll _relativerotation_pitch _relativerotation_yaw) (`KismetMathLibrary.BreakRotator` (`SceneComponent.RelativeRotation` _arrow)))
  ;[1 1 1] Snap To Rotation
  (for (_array_element _array_index) (`self.Setpoints`)
    (if (< (`KismetMathLibrary.Abs` (- _array_element (`self.CurrentRotation`))) (`self.Setpoint Sensitivity`))
      (bind _output_get (set `self.CurrentRotation` _array_element))
      (bind _location (`self.Parameterize Position` _output_get))
      (`SceneComponent.K2_SetRelativeRotation` _arrow (`KismetMathLibrary.MakeRotator` _location _relativerotation_pitch _relativerotation_yaw) false false)
      (set `self.FoundSnap` true)
      (bind _output_get_2 (set `self.SwitchValue` _array_index))
      (message `/Game/MachineBlueprints/MachineInterface.InputSpeedIntegerSelector` (`self.InteractionTarget`) _output_get_2)))
  ;;[1 1 1] If no snap, snap to earlier
  (if (`self.FoundSnap`)
    (set `self.FoundSnap` false)
    (else
      (goto _label))))

(event `self.HoldInteract`
  (params (MouseInput :type "Float (double-precision)"))
  (bind _arrow (`self.Arrow`))
  (bind _currentrotation (`self.CurrentRotation`))
  (bind (_relativerotation_roll _relativerotation_pitch _relativerotation_yaw) (`KismetMathLibrary.BreakRotator` (`SceneComponent.RelativeRotation` _arrow)))
  ;[1 1 1] Rotate with mouse
  (if true
    (if (not (or (and (>= MouseInput 0.0) (> _currentrotation 1.0)) (and (< _currentrotation 0.0) (<= MouseInput 0.0))))
      (bind _output_get (set `self.CurrentRotation` (+ (* MouseInput 0.01) (`self.CurrentRotation`))))
      (bind _location (`self.Parameterize Position` _output_get))
      (`SceneComponent.K2_SetRelativeRotation` _arrow (`KismetMathLibrary.MakeRotator` _location _relativerotation_pitch _relativerotation_yaw) false false))))

(fn `GetTooltip`
  (returns (`Text To Display` :type Text))
  (return (`self.TooltipText`)))

(fn `Parameterize Position`
  (params (Position :type "Float (double-precision)"))
  (returns (Location :type "Float (double-precision)"))
  (return (`KismetMathLibrary.Lerp` (`self.Rotation Minimum`) (`self.Rotation Maximum`) Position)))

(fn `UserConstructionScript`)