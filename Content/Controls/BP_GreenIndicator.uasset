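; BP_GreenIndicator is an indicator light that shows a pushed on/off state by glowing.
; The construction script creates a dynamic material instance from the Cube's first material.
; DisplayStatePush stores the received state and sets that material's Emissive parameter to EmissiveStrength when on, or zero when off.
; MachinePull returns only zero values, so the indicator supplies no data of its own.
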(event `/Game/MachineBlueprints/MachineInterface.DisplayStatePush`
  (params (StatePushed :type Boolean))
  (bind _dynamicmaterial (`self.DynamicMaterial`))
  ;[1 1 1] State Received
  (bind _output_get (set `self.Is on?` StatePushed))
  (if _output_get
    (`MaterialInstanceDynamic.SetScalarParameterValue` _dynamicmaterial "Emissive" (`self.EmissiveStrength`))
    (else
      (`MaterialInstanceDynamic.SetScalarParameterValue` _dynamicmaterial "Emissive" 0.0))))

(fn `MachinePull`
  (returns (IntegerData :type Integer) (FloatData :type "Float (double-precision)"))
  (return 0 0.0))

(fn `UserConstructionScript`
  (bind _cube (`self.Cube`))
  (bind _returnvalue (`PrimitiveComponent.CreateDynamicMaterialInstance` _cube 0 (`PrimitiveComponent.GetMaterial` _cube 0) "None"))
  (set `self.DynamicMaterial` _returnvalue))