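; BP_SwitchState is an interactable two-state switch that controls a linked machine and shows its state through a rotated arrow.
; Interact flips the SwitchState boolean, sends it to MahineInteract via InputStateSwitchMessage, then updates the arrow.
; BeginPlay applies the same instant rotation to match the initial state, without notifying the machine.
; GetTooltip returns the stored display tooltip.
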(event `self.ReceiveBeginPlay`
  (`SceneComponent.K2_SetRelativeRotation` (`self.Arrow`) (`KismetMathLibrary.SelectRotator` (struct :`Roll` 100.0) (struct) (stale `self.Interact` _output_get)) false true :!label _label))

(event `self.Interact`
  (bind _output_get (set `self.SwitchState` (not (`self.SwitchState`))))
  (message `/Game/MachineBlueprints/MachineInterface.InputStateSwitch` (`self.MahineInteract`) (`self.SwitchState`))
  (goto _label))

(fn `GetTooltip`
  (returns (`Text To Display` :type Text))
  (return (`self.TootltipToDisplay`)))

(fn `UserConstructionScript`)