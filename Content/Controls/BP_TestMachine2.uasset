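; BP_TestMachine2 is a test machine that pulls data from a linked Machine1 and pushes a computed result to a display target.
; Each tick it pushes the stored Result to DisplayTarget, then, while IsOn is set, recomputes it as the product of Machine1's float and integer data, otherwise zero.
; Its own MachinePull returns only zeros, and the logic that switches it off and loops over StateLights is unconnected.
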(event `self.ReceiveTick`
  (params (DeltaSeconds :type "Float (single-precision)"))
  (`self.DisplayPush`)
  (if (`self.IsOn?`)
    (bind (_integerdata _floatdata) (message `/Game/MachineBlueprints/MachineInterface.MachinePull` (`self.Machine1`))) ; Test
    (set `self.Result` (* _floatdata _integerdata))
    (else
      (set `self.Result` 0.0))))

(fn `DisplayPush`
  (message `/Game/MachineBlueprints/MachineInterface.DataPush` (`self.DisplayTarget`) (`self.Result`) 0))

(fn `MachinePull`
  (returns (IntegerData :type Integer) (FloatData :type "Float (double-precision)") (FloatData2 :type "Float (double-precision)"))
  (return 0 0.0 0.0))

(fn `UserConstructionScript`)