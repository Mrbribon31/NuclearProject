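; BP_TestMachine is a test machine that can be switched on and off, counting how often it turns on and how long it has been running.
; SwitchState sets the on state and forwards it to its StateLights.
; Tick pushes runtime and turn-on count to DataTargets every frame, accumulating time while on and zeroing it while off.
; MachinePull also returns both values on demand, offering pull alongside push.
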(event `/Game/MachineBlueprints/MachineInterface.SwitchState`
  (params (TurnOn :type Boolean))
  (bind _statelights (`self.StateLights`))
  ;[1 1 1] Changes State According To Input
  (if TurnOn
    (bind _output_get (set `self.IsOn?` true))
    (set `self.Times Turned On` (+ (`self.Times Turned On`) 1))
    (for _array_element _statelights
      (message `/Game/MachineBlueprints/MachineInterface.SwitchState` _array_element _output_get))
    (else
      (bind _output_get_2 (set `self.IsOn?` false))
      (for _array_element_2 _statelights
        (message `/Game/MachineBlueprints/MachineInterface.SwitchState` _array_element_2 _output_get_2)))))

(event `self.ReceiveTick`
  (params (DeltaSeconds :type "Float (single-precision)"))
  (`self.DisplayData`)
  (if (`self.IsOn?`)
    (set `self.MachineTime` (+ (`self.MachineTime`) DeltaSeconds))
    (else
      (set `self.MachineTime` 0.0))))

(fn `DisplayData`
  (for _array_element (`self.DataTargets`)
    (message `/Game/MachineBlueprints/MachineInterface.DataPush` _array_element (`self.MachineTime`) (`self.Times Turned On`))))

(fn `MachinePull`
  (returns (IntegerData :type Integer) (FloatData :type "Float (double-precision)"))
  (return (`self.Times Turned On`) (`self.MachineTime`)))

(fn `UserConstructionScript`)