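; BP_SwitchCrossover is an interactable two-state switch that controls a reactor crossover valve.
; Interacting toggles the state, and a SwitchState event sets it directly; both send the new value to MahineInteract as a crossover valve message.
; The Arrow component snaps between two rotations to show the state, which BeginPlay applies without sending a message.
; GetTooltip supplies its display text.
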(event `/Game/Controls/UpdateSwitchInterface.Switch State`
  (params (State :type Boolean))
  (bind _switchstate (`self.SwitchState`))
  (set `self.SwitchState` State)
  (message `/Game/MachineBlueprints/MachineInterface.InputReactorCrossoverValve` (`self.MahineInteract`) _switchstate :!label _label)
  (`SceneComponent.K2_SetRelativeRotation` (`self.Arrow`) (`KismetMathLibrary.SelectRotator` (struct :`Roll` 100.0) (struct) _switchstate) false true :!label _label_2))

(event `self.ReceiveBeginPlay`
  (goto _label_2))

(event `self.Interact`
  (set `self.SwitchState` (not (`self.SwitchState`)))
  (goto _label))

(fn `GetTooltip`
  (returns (`Text To Display` :type Text))
  (return (`self.TootltipToDisplay`)))

(fn `UserConstructionScript`)