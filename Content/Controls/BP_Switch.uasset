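; BP_Switch is an interactable two-state switch that controls a linked machine.
; Each Interact flips the boolean state, snaps the Arrow component between two relative rotations and passes the new state to MahineInteract through SwitchStateMessage.
; GetTooltip returns the stored tooltip for display.
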(event `/Game/FirstPerson/Blueprints/InteractInterface.Interact`
  (bind _output_get (set `self.SwitchState` (not (`self.SwitchState`))))
  (`SceneComponent.K2_SetRelativeRotation` (`self.Arrow`) (`KismetMathLibrary.SelectRotator` (struct :`Roll` 100.0) (struct) _output_get) false true)
  (message `/Game/MachineBlueprints/MachineInterface.SwitchState` (`self.MahineInteract`) (`self.SwitchState`)))

(fn `GetTooltip`
  (returns (`Text To Display` :type Text))
  (return (`self.TootltipToDisplay`)))

(fn `UserConstructionScript`)